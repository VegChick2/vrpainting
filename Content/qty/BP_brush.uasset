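; BP_brush is a grabbable paintbrush actor that paints on BP_Canvas in its assigned color.
; BeginPlay stores its start transform and tints the mesh, and dropping it returns it there.
; Each tick it line-traces between two tip components; any hit adds color rating over time to the level's canvas.
; If the hit actor is a canvas, it also calls OnPaint with the brush and hit.
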(event `self.GrabComponent.OnDropped`
  (`self.K2_SetActorTransform` self (`self.initialTransform`) false false))

(event `self.ReceiveBeginPlay`
  (set `self.initialTransform` (`self.GetTransform` self))
  (`PrimitiveComponent.CreateDynamicMaterialInstance` (`self.StaticMesh`) 0 "/Game/qty/MI_basic.MI_basic" "None")
  (`MeshComponent.SetVectorParameterValueOnMaterials` (`self.StaticMesh`) "color" (`KismetMathLibrary.Conv_LinearColorToVector` (`self.color`))))

(event `self.ReceiveTick`
  (params (DeltaSeconds :type "Float (single-precision)"))
  (bind (_outhit _returnvalue) (`KismetSystemLibrary.LineTraceSingleByProfile` (`SceneComponent.K2_GetComponentLocation` (`self.brushstart`)) (`SceneComponent.K2_GetComponentLocation` (`self.brushend`)) "BlockAllDynamic" true))
  (if _returnvalue
    (bind _returnvalue_2 (`GameplayStatics.GetActorOfClass` "/Game/qty/BP_Canvas.BP_Canvas_C"))
    (`/Game/qty/BP_Canvas.addRating` _returnvalue_2 (`KismetMathLibrary.Conv_LinearColorToVector` (`self.color`)) DeltaSeconds 1.0)
    (bind _asbp_canvas (cast `/Game/qty/BP_Canvas` (`.HitActor` (`GameplayStatics.BreakHitResult` _outhit))))
    (`/Game/qty/BP_Canvas.onPaint` _asbp_canvas self _outhit)))

(fn `UserConstructionScript`)