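; BP_Canvas is a paintable canvas actor that accumulates a colour-based rating of what is painted.
; On begin play or clear, it creates a render target for the plane's material and a brush material instance; clearing also zeroes the rating.
; Painting feeds hit UV and brush settings into that instance, then draws it to the render target.
; AddRating accumulates time-scaled colour; GetRating returns its truncated vector length, which Tick prints untruncated.
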(event `clearCanvas`
  (set `self.rating` (0.0 0.0 0.0))
  (bind _returnvalue (`PrimitiveComponent.CreateDynamicMaterialInstance` (`self.Plane`) 0 "/Game/qty/MI_Canvas.MI_Canvas" "None" :!label _label))
  (bind _returnvalue_2 (`KismetRenderingLibrary.CreateRenderTarget2D` 1024 1024))
  (set `self.renderToTexture` _returnvalue_2)
  (`MaterialInstanceDynamic.SetTextureParameterValue` _returnvalue "BrushStroke" _returnvalue_2)
  (bind _returnvalue_3 (`KismetMaterialLibrary.CreateDynamicMaterialInstance` "/Game/qty/MI_PaintBrush.MI_PaintBrush"))
  (set `self.BrushMaterialInstance` _returnvalue_3))

(event `self.ReceiveBeginPlay`
  (goto _label))

(event `self.ReceiveTick`
  (params (DeltaSeconds :type "Float (single-precision)"))
  (`KismetSystemLibrary.PrintString` (`KismetStringLibrary.Conv_DoubleToString` (`KismetMathLibrary.VSize` (`self.rating`)))))

(event `onPaint`
  (params (brush :type "/Game/qty/BP_brush Object Reference") (hit :type "HitResult Structure"))
  (bind _uv (`GameplayStatics.FindCollisionUV` hit))
  (set `self.Brush` brush)
  (`MaterialInstanceDynamic.SetVectorParameterValue` (`self.BrushMaterialInstance`) "HitPosition" (make `LinearColor` (`KismetMathLibrary.BreakVector2D` _uv) (`.Y` (`KismetMathLibrary.BreakVector2D` _uv)) 0.0 1.0))
  (`MaterialInstanceDynamic.SetVectorParameterValue` (`self.BrushMaterialInstance`) "BrushColor" (`/Game/qty/BP_brush.color` (`self.Brush`)))
  (`MaterialInstanceDynamic.SetScalarParameterValue` (`self.BrushMaterialInstance`) "BrushSize" (`/Game/qty/BP_brush.size` (`self.Brush`)))
  (`MaterialInstanceDynamic.SetScalarParameterValue` (`self.BrushMaterialInstance`) "BrushStrength" (`/Game/qty/BP_brush.strength` (`self.Brush`)))
  (`KismetRenderingLibrary.DrawMaterialToRenderTarget` (`self.renderToTexture`) (`self.BrushMaterialInstance`)))

(event `onPaintBullet`
  (bind _returnvalue (`GameplayStatics.GetActorOfClass` "/Game/qty/BP_brush_dummy.BP_brush_dummy_C"))
  (`self.onPaint` _returnvalue))

(fn `addRating`
  (params (color :type "Vector Structure") (deltatime :type "Float (double-precision)") (coeff :type "Float (double-precision)"))
  (set `self.rating` (+ (`self.rating`) (* color (* deltatime coeff)))))

(fn `getRating`
  (returns (rating :type Integer))
  (return (`KismetMathLibrary.FTrunc` (`KismetMathLibrary.VSize` (`self.rating`)))))

(fn `UserConstructionScript`)