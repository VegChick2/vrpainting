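; BP_curling is a grabbable, physics-driven curling object that paints the BP_Canvas beneath it and adds to that canvas's rating.
; Each tick a short downward trace from its cylinder passes the hit to the canvas, using a hidden BP_brush_dummy spawned far away to carry color, strength and size.
; Three seconds after being dropped it spawns an explosion, briefly doubles the brush size, then teleports to its starting transform and restarts physics.
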(event `self.ReceiveBeginPlay`
  (bind _textrender (`self.TextRender`))
  (set `self.initial Transform` (`self.GetTransform` self))
  (bind _returnvalue (`|SpawnActorFromClass` "/Game/qty/BP_brush_dummy.BP_brush_dummy_C" (`KismetMathLibrary.MakeTransform` (0.0 0.0 50000.0)) "Undefined" "OverrideRootScale" null null))
  (bind _output_get (set `self.Dummybrush` _returnvalue))
  (set `/Game/qty/BP_brush.color` (`self.Color`) _output_get)
  (set `/Game/qty/BP_brush.strength` (`self.Strength`) _output_get)
  (set `/Game/qty/BP_brush.size` (`self.Size`) _output_get)
  (`SceneComponent.SetVisibility` (`/Game/qty/BP_brush.StaticMesh` _returnvalue) false false)
  (`TextRenderComponent.K2_SetText` _textrender (`self.Value`))
  (`TextRenderComponent.SetTextRenderColor` _textrender (`KismetMathLibrary.Conv_LinearColorToColor` (`self.Color`))))

(event `self.ReceiveTick`
  (params (DeltaSeconds :type "Float (single-precision)"))
  (bind _returnvalue (`SceneComponent.K2_GetComponentLocation` (`self.Cylinder`)))
  (bind (_outhit _returnvalue_2) (`KismetSystemLibrary.LineTraceSingleByProfile` _returnvalue (+ _returnvalue (0.0 0.0 -15.0)) "BlockAllDynamic" true))
  (if _returnvalue_2
    (bind _asbp_canvas (cast `/Game/qty/BP_Canvas` (`.HitActor` (`GameplayStatics.BreakHitResult` _outhit))))
    (`/Game/qty/BP_Canvas.onPaint` _asbp_canvas (`self.Dummybrush`) _outhit)
    (`/Game/qty/BP_Canvas.addRating` _asbp_canvas (`KismetMathLibrary.Conv_LinearColorToVector` (`self.Color`)) DeltaSeconds 2.0)))

(event `self.GrabComponent.OnDropped`
  (`KismetSystemLibrary.K2_SetTimerDelegate` (delegate `CustomEvent_0`) 3.0))

(event `CustomEvent_0`
  (bind _cylinder (`self.Cylinder`))
  (`GameplayStatics.SpawnEmitterAtLocation` "/Game/StarterContent/Particles/P_Explosion.P_Explosion" (`self.K2_GetActorLocation`))
  (set `/Game/qty/BP_brush.size` (* (`self.Size`) 2.0) (`self.Dummybrush`))
  (`KismetSystemLibrary.Delay` 0.2)
  (`self.K2_SetActorTransform` self (`self.initial Transform`) false true)
  (`PrimitiveComponent.SetSimulatePhysics` _cylinder false)
  (`PrimitiveComponent.SetSimulatePhysics` _cylinder true)
  (set `/Game/qty/BP_brush.size` (`self.Size`) (`self.Dummybrush`)))

(fn `UserConstructionScript`)